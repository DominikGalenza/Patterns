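; BP_EliteUnit is an RTS unit that takes move and attack commands, backed by an AIC_EliteUnit controller cached on possession.
; SetMoveLocation stores the destination and writes it to the controller's MoveToLocation blackboard key, while StopMoving re-writes the stored destination unchanged.
; AttackTarget line-traces on the Visibility channel from the unit to the target, applying fixed damage on a direct hit and otherwise printing a no-line-of-sight message.
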(event EventPossessed
  (params (NewController :type Controller%20Object%20Reference))
  (bind _asaic_elite_unit (Utilities|Casting|CastToAIC_EliteUnit NewController))
  (Variables|Default|SetAIController _asaic_elite_unit))

(event EventSetMoveLocation
  (params (targetLocation :type Vector :default "0, 0, 0"))
  (bind _output_get (Variables|Default|SetMoveToLocation targetLocation))
  (AI|Components|Blackboard|SetValueasVector (AI|GetBlackboard (Variables|Default|GetAIController)) (Utilities|Name|MakeLiteralName "MoveToLocation") _output_get))

(event EventStopMoving
  (bind _output_get (Variables|Default|SetMoveToLocation (Variables|Default|GetMoveToLocation)))
  (AI|Components|Blackboard|SetValueasVector (AI|GetBlackboard (Variables|Default|GetAIController)) (Utilities|Name|MakeLiteralName "MoveToLocation") _output_get))

(event EventAttackTarget
  (params (target :type Object%20Object%20Reference))
  (bind _asactor (Utilities|Casting|CastToActor target))
  (bind _outhit (Collision|LineTraceByChannel (Transformation|GetActorLocation) (Transformation|GetActorLocation _asactor) "TraceTypeQuery1" false 0 "None"))
  (if (== (.HitActor (Collision|BreakHitResult _outhit)) target)
    (Game|Damage|ApplyDamage (.HitActor (Collision|BreakHitResult _outhit)) 1e+02 0 0)
    (else
      (Development|PrintString "No line of sight"))))

(fn ConstructionScript)